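; Samurai duelist actor with a paper sprite that slides into place on BeginPlay and takes a single draw attempt.
; Attack checks the phase in GM_Dual: pressing during Wait reveals a cross, while pressing during Draw lunges the sprite to AttackPos and swaps to the attack sprite.
; Either press sets PressedDraw to block further attempts, and both movements are timeline-driven lerps.
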(event Custom|SlideIn
  (Components|Timeline|SetPlayRate (Variables|Default|GetSlideInAnim) 1.5)
  (bind _alpha (Timeline|SlideInAnim PlayFromStart)
    (:Update
      (Transformation|SetRelativeLocation (Variables|Default|GetPaperSprite) (Math|Vector|Lerp(Vector) (Variables|Default|GetSlideStartPos) (Variables|Default|GetSpriteDefaultPos) _alpha) false false))))

(event Custom|Attack
  (if (not (Variables|Default|GetPressedDraw))
    (switch Utilities|FlowControl|Switch|SwitchonE_Phase (Variables|/Game/Blueprints/GM_Dual.GM_Dual_C|GetPhase (Variables|Default|GetGameMode))
      (:NewEnumerator1
        (CallFunction|SetCrossVisability true)
        (Variables|Default|SetPressedDraw true))
      (:NewEnumerator2
        (Variables|Default|SetPressedDraw true)
        (Components|Timeline|SetPlayRate (Variables|Default|GetAttackAnim) 8.0)
        (bind _alpha (Timeline|AttackAnim PlayFromStart)
          (:Update
            (Transformation|SetRelativeLocation (Variables|Default|GetPaperSprite) (Math|Vector|Lerp(Vector) (Variables|Default|GetSpriteDefaultPos) (Variables|/Script/Engine.SceneComponent|GetRelativeLocation (Variables|Default|GetAttack%20Pos)) _alpha) false false))
          (:SwitchSprite
            (Rendering|Components|Sprite|SetSprite (Variables|Default|GetPaperSprite) (Variables|Default|GetAttackSprite))))))))

(event EventBeginPlay
  (bind _asgm_dual (Utilities|Casting|CastToGM_Dual (Game|GetGameMode)))
  (Variables|Default|SetGameMode _asgm_dual)
  (Variables|Default|SetSpriteDefaultPos (Variables|/Script/Engine.SceneComponent|GetRelativeLocation (Variables|Default|GetPaperSprite)))
  (CallFunction|Slidein)
  (CallFunction|SetCrossVisability false))

(event Collision|EventActorBeginOverlap
  (params (OtherActor :type Actor%20Object%20Reference)))

(event EventTick
  (params (DeltaSeconds :type Float%20%28single-precision%29)))

(fn ConstructionScript)

(fn SetCrossVisability
  (params (bNewVisibility :type Boolean))
  (Rendering|SetVisibility (Variables|Default|GetCross) bNewVisibility false))